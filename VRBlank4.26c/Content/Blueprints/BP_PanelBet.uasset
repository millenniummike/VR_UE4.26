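; BP_PanelBet is a betting card panel that displays event name, bet type, participant, odds and sport as text, with a sport logo.
; SetCard fills each text field, then switches on the sport name to pick the Logo's material from the LogoMat array, with Football and Cricket having their own entries.
; The Panel event forwards only Sport to SetCard, and SetBetType updates the bet type text alone.
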(event Custom|Panel
  (params (Sport :type String))
  (CallFunction|SetCard "" "" "" "" Sport))

(fn ConstructionScript)

(fn SetCard
  (params (EventName :type String) (BetType :type String) (Participant :type String) (Odds :type String) (Sport :type String))
  (bind _returnvalue (Utilities|Text|ToText(String) Sport))
  (Rendering|Components|TextRender|SetText (Variables|Default|GetEventName) (Utilities|Text|ToText(String) EventName))
  (Rendering|Components|TextRender|SetText (Variables|Default|GetBetType) (Utilities|Text|ToText(String) BetType))
  (Rendering|Components|TextRender|SetText (Variables|Default|GetParticipant) (Utilities|Text|ToText(String) Participant))
  (Rendering|Components|TextRender|SetText (Variables|Default|GetOdds) (Utilities|Text|ToText(String) Odds))
  (Rendering|Components|TextRender|SetText (Variables|Default|GetSport) _returnvalue)
  (switch string (Utilities|String|ToString(Text) _returnvalue)
    (:Default
      (Variables|Default|SetLogoMatIndex 0))
    (:Football
      (Variables|Default|SetLogoMatIndex 1))
    (:Cricket
      (Variables|Default|SetLogoMatIndex 2)))
  (Rendering|Material|SetMaterial (Variables|Default|GetLogo) 0 (Utilities|Array|Get(acopy) (Variables|Default|GetLogoMat) (Variables|Default|GetLogoMatIndex))))

(fn SetBetType
  (params (BetType :type String))
  (Rendering|Components|TextRender|SetText (Variables|Default|GetBetType) (Utilities|Text|ToText(String) BetType)))