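; BP_ListenerLightToggle is an interactable button Actor that toggles the light direction flag on a LightController.
; Touch inverts the controller's IntensityUp boolean through a NOR with false, which acts as a NOT.
; Trigger, Pickup and Drop only print debug strings, with Pickup intended to be called by BP_MotionController.
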(event EventTouch
  (bind _lightcontroller (Variables|Default|GetLightController))
  (Development|PrintString "ButtonTouched")
  (Variables|/Game/Blueprints/BP_LightControl.BP_LightControl_C|SetIntensityUp _lightcontroller (Math|Boolean|NORBoolean (Variables|/Game/Blueprints/BP_LightControl.BP_LightControl_C|GetIntensityUp _lightcontroller) false)))

(event EventTrigger
  (params (SourceLocation :type Vector :default "0, 0, 0"))
  (Development|PrintString "ButtonTriggered"))

(event EventPickup
  (params (AttachTo :type Scene%20Component%20Object%20Reference))
  (Development|PrintString "Pickup!"))

(event EventDrop
  (Development|PrintString "Drop"))

(fn ConstructionScript)