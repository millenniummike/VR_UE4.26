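; Spawns a grid of BP_ListenerObject buttons that acts as a step-sequencer interface for a track in BPTrackPlayer.
; BeginPlay lays out the grid from the track's beat count, tags each button with track and step, then binds to BeatTick.
; Each tick refreshes highlights for the playback position and, with IfTrack, syncs button states and marks the track's position.
; Button triggers dispatch on ObjectID to toggle that step in the player.
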(event Custom|TriggerEvent
  (params (Actor :type Actor%20Object%20Reference))
  ;[1 1 1] Layout
  (bind _asbp_listener_object (Utilities|Casting|CastToBP_ListenerObject Actor))
  (Development|PrintString (Variables|/Game/Blueprints/BP_ListenerObject.BP_ListenerObject_C|GetObjectID _asbp_listener_object))
  (switch string (Variables|/Game/Blueprints/BP_ListenerObject.BP_ListenerObject_C|GetObjectID _asbp_listener_object)
    (:Test1
      (Default|ToggleTrackerBeat (Variables|Default|GetBP_TrackPlayer) (Variables|/Game/Blueprints/BP_ListenerObject.BP_ListenerObject_C|GetPayload _asbp_listener_object) (Variables|/Game/Blueprints/BP_ListenerObject.BP_ListenerObject_C|GetPayload2 _asbp_listener_object) (not (Variables|/Game/Blueprints/BP_ListenerObject.BP_ListenerObject_C|GetState _asbp_listener_object))))))

(event Custom|BeatTickeEvent
  (params (BeatNum :type Integer))
  (bind _bp_trackplayer (Variables|Default|GetBP_TrackPlayer))
  (bind _tracknumber (Variables|Default|GetTrackNumber))
  (bind _track (Variables|/Game/Blueprints/BP_TrackPlayer.BP_TrackPlayer_C|GetTrack _bp_trackplayer))
  (bind _output (Utilities|Array|Get(acopy) _track _tracknumber))
  (bind (_playonbeat _clip _trackbeatpos) (Utilities|Struct|BreakTrack _output))
  (Utilities|FlowControl|Sequence
    (:then_0
      ;[1 1 1] Unhiglight and set state
      (for (_array_element _array_index) (Variables|Default|GetButtons)
        (bind _asbp_listener_object (Utilities|Casting|CastToBP_ListenerObject _array_element))
        (Class|PickupActorInterface|UnHighlight(Message) _asbp_listener_object)
        (if (Variables|Default|GetIfTrack)
          (Variables|/Game/Blueprints/BP_ListenerObject.BP_ListenerObject_C|SetState _asbp_listener_object (Utilities|Array|Get(acopy) _playonbeat _array_index)))))
    (:then_1
      ;[1 1 1] Highlight Position
      (bind _asbp_listener_object_2 (Utilities|Casting|CastToBP_ListenerObject (Utilities|Array|Get(acopy) (Variables|Default|GetButtons) (/ (- BeatNum 1) (Variables|Default|GetBeatsInBar)))))
      (Class|PickupActorInterface|Highlight(Message) _asbp_listener_object_2))
    (:then_2
      ;[1 1 1] Highlight Track Position
      (if (Variables|Default|GetIfTrack)
        (bind _asbp_listener_object_3 (Utilities|Casting|CastToBP_ListenerObject (Utilities|Array|Get(acopy) (Variables|Default|GetButtons) _trackbeatpos)))
        (Class|PickupActorInterface|Highlight(Message) _asbp_listener_object_3)))))

(event EventBeginPlay
  (bind _returnvalue (Transformation|GetActorLocation))
  ;[1 1 1] Setup
  (Utilities|FlowControl|Sequence
    (:then_0
      (Variables|Default|SetStartX (.x _returnvalue))
      (Variables|Default|SetStartY (.y _returnvalue))
      (Variables|Default|SetStartZ (.z _returnvalue))
      (Variables|Default|SetMaxX (/ (.TrackBeatsInBar (Utilities|Struct|BreakTrack (Utilities|Array|Get(acopy) (Variables|/Game/Blueprints/BP_TrackPlayer.BP_TrackPlayer_C|GetTrack (Variables|Default|GetBP_TrackPlayer)) (Variables|Default|GetTrackNumber)))) (Variables|Default|GetMaxY)))
      ;[1 1 1] Layout
      (while (< (Variables|Default|GetCurrentY) (Variables|Default|GetMaxY)) :!label _label
        (while (< (Variables|Default|GetCurrentX) (Variables|Default|GetMaxX))
          (bind _returnvalue_2 (Game|SpawnActorfromClass "/Game/Blueprints/BP_ListenerObject.BP_ListenerObject_C" (Math|Transform|MakeTransform (Math|Vector|MakeVector (+ (* (stale _output_get) (Variables|Default|GetSpacingX)) (Variables|Default|GetStartX)) (+ (* (stale _output_get_2) (Variables|Default|GetSpacingY)) (Variables|Default|GetStartY)) (Variables|Default|GetStartZ)) "0, 0, 0" "0.250000,0.250000,0.100000") "Undefined" 0 0))
          (bind _output_get (Variables|Default|SetCurrentX (+ (Variables|Default|GetCurrentX) 1)))
          (bind _asbp_listener_object (Utilities|Casting|CastToBP_ListenerObject _returnvalue_2))
          (Variables|/Game/Blueprints/BP_ListenerObject.BP_ListenerObject_C|SetObjectID _asbp_listener_object (Variables|Default|GetObject%20ID))
          (Variables|/Game/Blueprints/BP_ListenerObject.BP_ListenerObject_C|SetPayload _asbp_listener_object (Variables|Default|GetTrackNumber))
          (Variables|/Game/Blueprints/BP_ListenerObject.BP_ListenerObject_C|SetPayload2 _asbp_listener_object (Variables|Default|GetPayload))
          (Variables|Default|SetPayload (+ (Variables|Default|GetPayload) 1))
          (EventDispatchers|BindEventtoTriggerEvent _asbp_listener_object (delegate Custom|TriggerEvent))
          (Utilities|Array|Add (Variables|Default|GetButtons) _asbp_listener_object))
        (Variables|Default|SetCurrentX 0)
        (bind _output_get_2 (Variables|Default|SetCurrentY (+ (Variables|Default|GetCurrentY) 1)))
        (goto _label)))
    (:then_1
      (EventDispatchers|BindEventtoBeatTick (Variables|Default|GetBP_TrackPlayer) (delegate Custom|BeatTickeEvent)))))

(fn ConstructionScript)