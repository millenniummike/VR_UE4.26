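; TimeSynth-based music Blueprint that plays clips in time with a metronome and mixes low and high intensity volume groups.
; Each beat tick advances a wrapping step counter and, if Track1 is on and that step is set, plays its clip in the DoriansRun_Lo group.
; High intensity volume uses a sine curve to map normalized input to decibels, then both groups are set without fades.
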(event Custom|BeatTickeEvent
  (params (BeatNum :type Integer))
  ;[1 1 1] Process Beats
  (Variables|Default|SetbeatNum (+ (Variables|Default|GetbeatNum) 1))
  (if (>= (Variables|Default|GetbeatNum) (Variables|Default|GetbeatsInBar))
    (Variables|Default|SetbeatNum 0))
  (if (Utilities|Array|Get(acopy) (Variables|Default|GetTrack1) (Variables|Default|GetbeatNum))
    (if (Variables|Default|GetTrack1On)
      (Class|TimeSynthComponent|PlayClip (Variables|Default|GetTimeSynth) (Variables|Default|GetTrack1Clip) "/Game/VolumeGroups/DoriansRun_Lo.DoriansRun_Lo"))))

(event Custom|OnBarEvent
  (params (QuantizationType :type ETimeSynthEventQuantization%20Enum :default "None") (NumBars :type Integer) (Beat :type Float%20%28single-precision%29))
  (Variables|Default|SetbarNum (+ (Variables|Default|GetbarNum) 1)))

(event EventBeginPlay
  (EventDispatchers|BindEventtoBeatTick (Variables|Default|GetMetronome) (delegate Custom|BeatTickeEvent)))

(fn ConstructionScript)

(fn SetHighIntensityVolume
  (params (NormalizedIn :type Float%20%28single-precision%29))
  ;[1 1 1] Non-Linear Mapping of Normalized to non-Normalized dB values.
  (Variables|Default|SetHighIntensityVolumeDB (Math|Float|MapRangeClamped (Math|Trig|Sin(Radians) (* NormalizedIn (Math|Float|MultiplybyPi 0.5))) 0.0 1.0 -6e+01 0.0))
  (CallFunction|SetVolumeGroups))

(fn SetVolumeGroups
  (Class|TimeSynthComponent|SetVolumeGroup (Variables|Default|GetTimeSynth) 0 (Variables|Default|GetLowIntensityVolumeDB) 0.0)
  (Class|TimeSynthComponent|SetVolumeGroup (Variables|Default|GetTimeSynth) 0 (Variables|Default|GetHighIntensityVolumeDB) 0.0))

(fn UpdateProgressBars)