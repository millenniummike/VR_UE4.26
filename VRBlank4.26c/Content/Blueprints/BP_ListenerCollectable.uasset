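; BP_ListenerCollectable is a physics collectable that launches itself toward a source location when triggered and can be picked up by BP_MotionController.
; Trigger computes a custom-arc projectile velocity from the static mesh to that location and applies it as the mesh's physics velocity.
; Hit forwards the other actor to CallCollisionEvent with an empty object ID.
; Touch, Pickup and Drop only print debug messages.
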(event EventTrigger
  (params (SourceLocation :type Vector :default "0, 0, 0"))
  (bind _outlaunchvelocity (Game|SuggestProjectileVelocityCustomArc (Transformation|GetWorldLocation (Variables|Default|GetStaticMeshComponent)) SourceLocation 0.0 0.5))
  (Class|PrimitiveComponent|SetAllPhysicsLinearVelocity (Variables|Default|GetStaticMeshComponent) _outlaunchvelocity false))

(event EventPickup
  (params (AttachTo :type Scene%20Component%20Object%20Reference))
  (Development|PrintString "Pickup!"))

(event Collision|EventHit
  (params (MyComp :type Primitive%20Component%20Object%20Reference) (Other :type Actor%20Object%20Reference) (OtherComp :type Primitive%20Component%20Object%20Reference) (bSelfMoved :type Boolean) (HitLocation :type Vector :default "0, 0, 0") (HitNormal :type Vector :default "0, 0, 0") (NormalImpulse :type Vector :default "0, 0, 0") (Hit :type Hit%20Result%20Structure%20%28by%20ref%29))
  (Default|CallCollisionEvent Other))

(event EventDrop
  (Development|PrintString "Drop"))

(event EventTouch
  (Development|PrintString "Touch"))

(fn ConstructionScript)