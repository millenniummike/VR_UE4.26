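; BP_ListenerBox is an interactable box that relays hit, touch and trigger events through collision and trigger event calls, and can be picked up by BP_MotionController.
; Touch toggles a highlight material, which Highlight and UnHighlight also set directly.
; When unhighlighted, as at BeginPlay, the State flag selects the on or original material.
; Pickup and Drop only print, and an ObjectID check that destroys the actor is unconnected.
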(event EventHighlight
  (Rendering|Material|SetMaterial (Variables|Debug|GetStaticMeshComponent) 0 (Variables|Default|GetHighlightMaterial)))

(event EventUnHighlight
  (bind _staticmeshcomponent (Variables|Debug|GetStaticMeshComponent))
  (if (Variables|Default|GetState)
    (Rendering|Material|SetMaterial _staticmeshcomponent 0 (Variables|Default|GetOnMaterial))
    (else
      (Rendering|Material|SetMaterial _staticmeshcomponent 0 (Variables|Default|GetOrigMaterial)))))

(event EventBeginPlay
  (bind _staticmeshcomponent (Variables|Debug|GetStaticMeshComponent))
  (if (Variables|Default|GetState)
    (Rendering|Material|SetMaterial _staticmeshcomponent 0 (Variables|Default|GetOnMaterial))
    (else
      (Rendering|Material|SetMaterial _staticmeshcomponent 0 (Variables|Default|GetOrigMaterial)))))

(event EventPickup
  (params (AttachTo :type Scene%20Component%20Object%20Reference))
  (Development|PrintString "Pickup!"))

(event Collision|EventHit
  (params (MyComp :type Primitive%20Component%20Object%20Reference) (Other :type Actor%20Object%20Reference) (OtherComp :type Primitive%20Component%20Object%20Reference) (bSelfMoved :type Boolean) (HitLocation :type Vector :default "0, 0, 0") (HitNormal :type Vector :default "0, 0, 0") (NormalImpulse :type Vector :default "0, 0, 0") (Hit :type Hit%20Result%20Structure%20%28by%20ref%29))
  (Default|CallCollisionEvent Other))

(event EventDrop
  (Development|PrintString "Drop"))

(event EventTouch
  (bind _staticmeshcomponent (Variables|Debug|GetStaticMeshComponent))
  (Development|PrintString "Touch")
  (Default|CallTriggerEvent self)
  (Variables|Default|SetHighlighted (not (Variables|Default|GetHighlighted)))
  (if (Variables|Default|GetHighlighted)
    (Rendering|Material|SetMaterial _staticmeshcomponent 0 (Variables|Default|GetHighlightMaterial))
    (elif (Variables|Default|GetState)
      (Rendering|Material|SetMaterial _staticmeshcomponent 0 (Variables|Default|GetOnMaterial))
      (else
        (Rendering|Material|SetMaterial _staticmeshcomponent 0 (Variables|Default|GetOrigMaterial))))))

(event EventTrigger
  (params (SourceLocation :type Vector :default "0, 0, 0"))
  (Development|PrintString "Trigger")
  (Default|CallTriggerEvent self))

(fn ConstructionScript)