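; VR game controller that routes motion controller input to pawn movement, a menu panel and interactive objects.
; On BeginPlay it binds handlers to every BP_MotionController event and stores the left one, whose hand direction steers jet movement on Tick.
; Controlled, held and touched BP_ListenerObjects receive highlight, trigger or touch messages, with touched ObjectIDs setting HoldingItem.
; The menu panel spawns once, then gets repositioned, closing by moving to world origin.
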(event Custom|MenuButtonEvent
  (params (Transform :type Transform) (On :type Boolean))
  ;[1 1 1] Handle Menu
  (Development|PrintString "Menu Button Event")
  (if On
    (CallFunction|OpenMenu (.location Transform) (.rotation Transform))
    (else
      (CallFunction|CloseMenu))))

(event Custom|SpawnEvent
  (params (Location :type Vector))
  ;[1 1 1] Handle Spawn Event
  (Development|PrintString "Spawn Event"))

(event Custom|SetHeldObject
  (params (Actor :type Actor%20Object%20Reference))
  ;[1 1 1] Held Logic
  (Variables|Default|SetHeldActor Actor))

(event Custom|JetEvent
  (params (State :type Boolean))
  (Variables|Default|SetJetEnabled State))

(event Custom|TurnEvent
  (params (ZDirection :type Integer))
  (bind _returnvalue (Math|Conversions|ToFloat(Integer) ZDirection))
  ;[1 1 1] Handle Turn
  (Transformation|AddActorLocalRotation (Variables|Default|GetPawn) (Math|Rotator|MakeRotator 0.0 0.0 _returnvalue) false false)
  (Development|PrintString (Utilities|String|ToString(Float) _returnvalue)))

(event Custom|SetControlledActor
  (params (Actor :type Actor%20Object%20Reference))
  ;[1 1 1] Handle Controlled Object
  (bind _asbp_listener_object (Utilities|Casting|CastToBP_ListenerObject (Variables|Default|GetControlledActor))
    (:then
      (Class|PickupActorInterface|UnHighlight(Message) _asbp_listener_object))
    (:CastFailed
      _))
  (bind _output_get (Variables|Default|SetControlledActor Actor))
  (bind _asbp_listener_object_2 (Utilities|Casting|CastToBP_ListenerObject _output_get))
  (Class|PickupActorInterface|Highlight(Message) _asbp_listener_object_2))

(event Custom|OverlapEvent
  (params (Actor :type Actor%20Object%20Reference))
  ;[1 1 1] Handle Overlap Event
  (CallFunction|TouchLogic Actor (stale EventBeginPlay _array_element)))

(event Custom|TriggerControlledActor
  (params (Location :type Vector))
  ;[1 1 1] Handle Controlled Object
  (CallFunction|TriggerLogic (Variables|Default|GetControlledActor) Location))

(event Custom|TestEvent
  (Development|PrintString "TestEvent")
  (CallFunction|OpenMenu "0, 0,330.000000" "0, 0, 0"))

(event Custom|TestEvent2
  (Development|PrintString "TestEvent2")
  (CallFunction|CloseMenu))

(event Custom|EventTriggerHeldObject
  ;[1 1 1] Held Logic
  (Development|PrintString "*************************")
  (Class|PickupActorInterface|Trigger(Message) (Variables|Default|GetHeldActor) "0, 0, 0"))

(event Custom|TestEvent3
  (CallFunction|TriggerLogic (Variables|Default|GetHeldActor) "0, 0, 0"))

(event EventBeginPlay
  (Utilities|FlowControl|Delay 0.0)
  (Development|PrintString "Binding")
  (Utilities|FlowControl|Sequence
    (:then_0
      ;[1 1 1] Bind Controllers
      (bind _outactors (Actor|GetAllActorsOfClass "/Game/VirtualRealityBP/Blueprints/BP_MotionController.BP_MotionController_C"))
      (for _array_element _outactors
        (Utilities|FlowControl|Sequence
          (:then_0
            ;[1 1 1] Handle Controlled Object
            (EventDispatchers|BindEventtoSetControlObjectEvent _array_element (delegate Custom|SetControlledActor)))
          (:then_1
            ;[1 1 1] Handle Spawn Event
            (EventDispatchers|BindEventtoSpawnEvent _array_element (delegate Custom|SpawnEvent)))
          (:then_2
            ;[1 1 1] Handle Menu
            (EventDispatchers|BindEventtoMenuButtonEvent _array_element (delegate Custom|MenuButtonEvent)))
          (:then_3
            ;[1 1 1] Handle Turn
            (EventDispatchers|BindEventtoTurn _array_element (delegate Custom|TurnEvent)))
          (:then_4
            ;[1 1 1] Handle Overlap Event
            (EventDispatchers|BindEventtoOverlapEvent _array_element (delegate Custom|OverlapEvent)))
          (:then_5
            (if true
              (EventDispatchers|BindEventtoTriggerControlledObject _array_element (delegate Custom|TriggerControlledActor))))
          (:then_6
            ;[1 1 1] Held Logic
            (EventDispatchers|BindEventtoTriggerHeldObject _array_element (delegate Custom|EventTriggerHeldObject))
            (EventDispatchers|BindEventtoSetHeldOjbect _array_element (delegate Custom|SetHeldObject)))
          (:then_7
            (EventDispatchers|BindEventtoJet _array_element (delegate Custom|JetEvent)))
          (:then_8
            (if (Utilities|Enum|Equal(Enum) (Variables|/Game/VirtualRealityBP/Blueprints/BP_MotionController.BP_MotionController_C|GetHand _array_element) "Left")
              (Variables|Default|SetControllerLeft _array_element))))))))

(event EventTick
  (params (DeltaSeconds :type Float%20%28single-precision%29))
  (if (Variables|Default|GetJetEnabled)
    (bind _asbp_motion_controller (Utilities|Casting|CastToBP_MotionController (Variables|Default|GetControllerLeft)))
    (Transformation|AddActorWorldOffset (Variables|Default|GetPawn) (* (Math|Vector|GetForwardVector (Variables|/Game/VirtualRealityBP/Blueprints/BP_MotionController.BP_MotionController_C|GetHandMesh _asbp_motion_controller)) (Variables|Default|GetJetSpeed)))))

(fn ConstructionScript)

(fn TriggerLogic
  (params (Actor :type Actor%20Object%20Reference) (SourceLocation :type Vector))
  (Development|PrintString "TriggerLogic")
  (bind _asbp_listener_object (Utilities|Casting|CastToBP_ListenerObject Actor))
  (Class|PickupActorInterface|Trigger(Message) _asbp_listener_object SourceLocation)
  (switch string (Variables|/Game/Blueprints/BP_ListenerObject.BP_ListenerObject_C|GetObjectID _asbp_listener_object)))

(fn OpenMenu
  (params (Location :type Vector) (Rotation :type Rotator))
  (Development|PrintString "Open Menu")
  (Utilities|Casting|CastToBP_MenuPanel (Variables|Default|GetMenu)
    (:then
      (Transformation|SetActorLocation (Variables|Default|GetMenu) Location false false))
    (:CastFailed
      (bind _returnvalue (Game|SpawnActorfromClass "/Game/Blueprints/BP_MenuPanel.BP_MenuPanel_C" (Math|Transform|MakeTransform Location Rotation "1,1,1") "Undefined" 0 0))
      (bind _output_get (Variables|Default|SetMenu _returnvalue))))
  (Transformation|SetActorRotation (Variables|Default|GetMenu) (Math|Rotator|MakeRotator 0.0 0.0 (+ (.Yaw (Math|Rotator|BreakRotator Rotation)) 9e+01)))
  (Transformation|AddLocalOffset (Variables|/Script/Engine.Actor|GetRootComponent _output_get) "0,-20.000000, 0" false false))

(fn CloseMenu
  (Transformation|SetActorLocation (Variables|Default|GetMenu) "0, 0, 0" false false))

(fn TouchLogic
  (params (Actor :type Actor%20Object%20Reference) (MotionController :type Actor%20Object%20Reference))
  (bind _asbp_listener_object (Utilities|Casting|CastToBP_ListenerObject Actor))
  (Class|PickupActorInterface|Touch(Message) _asbp_listener_object)
  (bind _asbp_motion_controller (Utilities|Casting|CastToBP_MotionController MotionController))
  (switch string (Variables|/Game/Blueprints/BP_ListenerObject.BP_ListenerObject_C|GetObjectID _asbp_listener_object)
    (:Nothing
      (Variables|/Game/VirtualRealityBP/Blueprints/BP_MotionController.BP_MotionController_C|SetHoldingItem _asbp_motion_controller 0))
    (:Gun1
      (Variables|/Game/VirtualRealityBP/Blueprints/BP_MotionController.BP_MotionController_C|SetHoldingItem _asbp_motion_controller 1))
    (:Gun2
      (Variables|/Game/VirtualRealityBP/Blueprints/BP_MotionController.BP_MotionController_C|SetHoldingItem _asbp_motion_controller 2))))