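; BP_TrackPlayer is a TimeSynth step sequencer that plays clips from per-track beat patterns, editable at runtime through ToggleTrackerBeat.
; Quantization delegates drive bar and sixteenth-note counters, text readouts and a BeatTick broadcast.
; Each sixteenth advances every track's wrapping position and fires clips on active steps, all into the DoriansRun_Lo volume group.
; Low and high intensity volume groups are set in dB, with high intensity mapped from normalized input along a sine curve.
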(event Custom|On1/16
  (params (QuantizationType :type ETimeSynthEventQuantization%20Enum :default "None") (NumBars :type Integer) (Beat :type Float%20%28single-precision%29))
  (bind _track (Variables|Default|GetTrack))
  (bind _output_get (Variables|Default|SetbeatNum (+ (Variables|Default|GetbeatNum) 1)))
  (Rendering|Components|TextRender|SetText (Variables|Default|GetBeat) (Utilities|Text|ToText(Integer) _output_get))
  (Default|CallBeatTick _output_get)
  (for (_ _array_index) _track
    (if (>= (+ (.trackbeatpos (Utilities|Array|Get(acopy) _track _array_index)) 1) (.trackbeatsinbar (Utilities|Array|Get(acopy) _track _array_index)))
      (Utilities|Array|SetArrayElem _track _array_index (Utilities|Struct|MakeTrack (.playonbeat (Utilities|Array|Get(acopy) _track _array_index)) (.clip (Utilities|Array|Get(acopy) _track _array_index)) 0 (.trackbeatsinbar (Utilities|Array|Get(acopy) _track _array_index))))
      (else
        (Utilities|Array|SetArrayElem _track _array_index (Utilities|Struct|MakeTrack (.playonbeat (Utilities|Array|Get(acopy) _track _array_index)) (.clip (Utilities|Array|Get(acopy) _track _array_index)) (+ (.trackbeatpos (Utilities|Array|Get(acopy) _track _array_index)) 1) (.trackbeatsinbar (Utilities|Array|Get(acopy) _track _array_index))))))
    (if (Utilities|Array|Get(acopy) (.playonbeat (Utilities|Array|Get(acopy) _track _array_index)) (.trackbeatpos (Utilities|Array|Get(acopy) _track _array_index)))
      (Class|TimeSynthComponent|PlayClip (Variables|Default|GetTimeSynth) (.clip (Utilities|Array|Get(acopy) _track _array_index)) "/Game/VolumeGroups/DoriansRun_Lo.DoriansRun_Lo"))))

(event Custom|ToggleTrackerBeat
  (params (TrackNum :type Integer) (BeatNum :type Integer) (State :type Boolean))
  (bind _track (Variables|Default|GetTrack))
  (bind _output_get (Variables|Default|SetCurrentTrack (Utilities|Array|Get(acopy) _track TrackNum)))
  (Utilities|Array|SetArrayElem (.PlayOnBeat (Utilities|Struct|BreakTrack _output_get)) BeatNum State)
  (Utilities|Array|SetArrayElem _track TrackNum (Variables|Default|GetCurrentTrack))
  (Development|PrintString "Updated Tracker"))

(event Custom|OnBarEvent
  (params (QuantizationType :type ETimeSynthEventQuantization%20Enum :default "None") (NumBars :type Integer) (Beat :type Float%20%28single-precision%29))
  (bind _output_get (Variables|Default|SetbarNum (+ (Variables|Default|GetbarNum) 1)))
  (Rendering|Components|TextRender|SetText (Variables|Default|GetBar) (Utilities|Text|ToText(String) (Utilities|String|ToString(Integer) _output_get)))
  (Variables|Default|SetbeatNum 0))

(event EventBeginPlay
  (Components|Activation|Activate (Variables|Default|GetTimeSynth) false)
  ;[1 1 1] Set up Quantization Delegates
  (Class|TimeSynthComponent|AddQuantizationEventDelegate (Variables|Default|GetTimeSynth) "Bars4" (EventDispatchers|CreateEvent :!event Custom|OnBarEvent))
  (Class|TimeSynthComponent|AddQuantizationEventDelegate (Variables|Default|GetTimeSynth) "SixteenthNote" (EventDispatchers|CreateEvent :!event Custom|On1/16))
  (CallFunction|SetVolumeGroups))

(fn ConstructionScript)

(fn SetHighIntensityVolume
  (params (NormalizedIn :type Float%20%28single-precision%29))
  ;[1 1 1] Non-Linear Mapping of Normalized to non-Normalized dB values.
  (Variables|Default|SetHighIntensityVolumeDB (Math|Float|MapRangeClamped (Math|Trig|Sin(Radians) (* NormalizedIn (Math|Float|MultiplybyPi 0.5))) 0.0 1.0 -6e+01 0.0))
  (CallFunction|SetVolumeGroups))

(fn SetVolumeGroups
  (Class|TimeSynthComponent|SetVolumeGroup (Variables|Default|GetTimeSynth) 0 (Variables|Default|GetLowIntensityVolumeDB) 0.0)
  (Class|TimeSynthComponent|SetVolumeGroup (Variables|Default|GetTimeSynth) 0 (Variables|Default|GetHighIntensityVolumeDB) 0.0))

(fn UpdateProgressBars)