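; BP_SlotMachine is a slot machine Blueprint that animates three spinning reels.
; Each tick, a sequence checks a spinning flag per reel and adds that reel's speed to its component's relative rotation.
; The speed is applied per frame without delta-time scaling, and nothing in these graphs sets the flags, stops the reels or evaluates results.
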(event EventTick
  (params (DeltaSeconds :type Float%20%28single-precision%29))
  (Utilities|FlowControl|Sequence
    (:then_0
      (if (Variables|Default|GetReel1Spinning)
        (Transformation|AddRelativeRotation (Variables|Default|GetBPReel) (Variables|Default|GetReel1Speed) false false)))
    (:then_1
      (if (Variables|Default|GetReel2Spinning)
        (Transformation|AddRelativeRotation (Variables|Default|GetBPReel1) (Variables|Default|GetReel2Speed) false false)))
    (:then_2
      (if (Variables|Default|GetReel3Spinning)
        (Transformation|AddRelativeRotation (Variables|Default|GetBPReel2) (Variables|Default|GetReel3Speed) false false)))))

(fn ConstructionScript)