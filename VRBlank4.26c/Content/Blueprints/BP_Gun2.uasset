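; BP_Gun2 is a gun actor for motion-controller interaction that fires BP_ListenerCone actors as physical projectiles.
; Trigger spawns a cone at the LaunchLocation component's transform and launches it with a mass-dependent impulse along that component's forward vector, scaled by ProjectTileSpeed.
; Pickup, called by BP_MotionController, and Drop only print debug messages, while Touch is empty.
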(event EventTrigger
  (params (SourceLocation :type Vector :default "0, 0, 0"))
  (bind _launchlocation (Variables|Default|GetLaunchLocation))
  (Development|PrintString "FIRE!")
  (bind _returnvalue (Game|SpawnActorfromClass "/Game/Blueprints/BP_ListenerCone.BP_ListenerCone_C" (Math|Transform|MakeTransform (Transformation|GetWorldLocation _launchlocation) (Transformation|GetWorldRotation _launchlocation) "1,1,1") "Undefined" 0 0))
  (Physics|AddImpulse (Variables|/Script/Engine.StaticMeshActor|GetStaticMeshComponent _returnvalue) (* (Math|Vector|GetForwardVector _launchlocation) (Variables|Default|GetProjectTileSpeed)) "None" false))

(event EventPickup
  (params (AttachTo :type Scene%20Component%20Object%20Reference))
  (Development|PrintString "Pickup!"))

(event EventDrop
  (Development|PrintString "Drop"))

(event EventTouch)

(fn ConstructionScript)