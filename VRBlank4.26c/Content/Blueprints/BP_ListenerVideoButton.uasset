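; BP_ListenerVideoButton is a VR interactable button that loads a web video on a target video panel when touched.
; Its Touch event copies its WebViewUrl into the panel's Webview1URL and calls LoadVideo.
; Trigger, Pickup and Drop only print debug messages, with Pickup noted as called by BP_MotionController.
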(event EventTouch
  (bind _targetvideopanel (Variables|Default|GetTargetVideoPanel))
  (Development|PrintString "ButtonTouched")
  (Variables|/Game/Blueprints/BP_VideoPanel.BP_VideoPanel_C|SetWebview1URL _targetvideopanel (Variables|Default|GetWebViewUrl))
  (Default|LoadVideo _targetvideopanel))

(event EventTrigger
  (params (SourceLocation :type Vector :default "0, 0, 0"))
  (Development|PrintString "ButtonTriggered"))

(event EventPickup
  (params (AttachTo :type Scene%20Component%20Object%20Reference))
  (Development|PrintString "Pickup!"))

(event EventDrop
  (Development|PrintString "Drop"))

(fn ConstructionScript)