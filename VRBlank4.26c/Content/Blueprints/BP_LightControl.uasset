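; BP_LightControl is a Blueprint that fades the intensity of a referenced Light up or down.
; On BeginPlay it caches the light's current intensity as the starting value.
; Each Tick it steps that value by Inc according to the IntensityUp flag, clamps it at TargetLightIntensity or zero, and applies it to the light component.
; The step ignores delta time, so fade speed depends on frame rate.
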(event EventBeginPlay
  (Variables|Default|SetCurrent%20Light%20Intensity (Variables|/Script/Engine.LightComponentBase|GetIntensity (Variables|/Script/Engine.Light|GetLightComponent (Variables|Default|GetLight)))))

(event EventTick
  (params (DeltaSeconds :type Float%20%28single-precision%29))
  (bind _light (Variables|Default|GetLight))
  (bind _lightcomponent (Variables|/Script/Engine.Light|GetLightComponent _light))
  (if (Variables|Default|GetIntensityUp)
    (Variables|Default|SetCurrent%20Light%20Intensity (+ (Variables|Default|GetCurrent%20Light%20Intensity) (Variables|Default|GetInc)))
    (if (> (Variables|Default|GetCurrent%20Light%20Intensity) (Variables|Default|GetTarget%20Light%20Intensity))
      (bind _output_get (Variables|Default|SetCurrent%20Light%20Intensity (Variables|Default|GetTarget%20Light%20Intensity))))
    (Rendering|Components|Light|SetIntensity _lightcomponent _output_get)
    (else
      (Variables|Default|SetCurrent%20Light%20Intensity (- (Variables|Default|GetCurrent%20Light%20Intensity) (Variables|Default|GetInc)))
      (if (< (Variables|Default|GetCurrent%20Light%20Intensity) 0.0)
        (bind _output_get_2 (Variables|Default|SetCurrent%20Light%20Intensity 0.0)))
      (Rendering|Components|Light|SetIntensity _lightcomponent _output_get_2))))

(event Collision|EventActorBeginOverlap
  (params (OtherActor :type Actor%20Object%20Reference)))

(fn ConstructionScript)